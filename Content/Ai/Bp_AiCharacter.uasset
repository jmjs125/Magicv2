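; AI enemy character that mirrors its health into an EnemyHealth widget, set on BeginPlay and refreshed every Tick.
; Tick also shows a cube once the enemy is hit, moves its box to the mesh's location and caches its owner as a defend point.
; InRange is a test jump that launches the character toward a nav location, using math expressions to derive velocity from jump time and gravity.
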(event Custom|update%20health
  (bind _enemy_health (Variables|Default|GetEnemy%20health))
  (Variables|/Game/UI/Enemy/EnemyHealth.EnemyHealth_C|Setmax%20health _enemy_health (Variables|Default|GetMaxHealth))
  (Variables|/Game/UI/Enemy/EnemyHealth.EnemyHealth_C|Sethealth _enemy_health (Variables|Default|GetHealth)))

(event EventBeginPlay
  (bind _asenemy_health (Utilities|Casting|CastToEnemyHealth (UserInterface|GetUserWidgetObject (Variables|Default|GetWidget))))
  (bind _output_get (Variables|Default|SetEnemy%20health _asenemy_health))
  (Variables|/Game/UI/Enemy/EnemyHealth.EnemyHealth_C|Setmax%20health _output_get (Variables|Default|GetMaxHealth))
  (Variables|/Game/UI/Enemy/EnemyHealth.EnemyHealth_C|Sethealth (Variables|Default|GetEnemy%20health) (Variables|Default|GetHealth)))

(event Collision|EventActorBeginOverlap
  (params (OtherActor :type Actor%20Object%20Reference)))

(event EventTick
  (params (DeltaSeconds :type Float%20%28single-precision%29))
  (Utilities|FlowControl|Sequence
    (:then_0
      (if (Variables|Default|GetEnemyBeenHit)
        (Rendering|SetVisibility (Variables|Default|GetCube) true false)))
    (:then_1
      (Transformation|SetRelativeLocation (Variables|Default|GetBox) (Transformation|GetWorldLocation (Variables|Character|GetMesh)) false false))
    (:then_2
      (bind _asbp_defendpoint (Utilities|Casting|CastTobp_Defendpoint (Components|GetOwner)))
      (Variables|Default|SetAs%20Bp%20Defendpoint _asbp_defendpoint))
    (:then_3
      (CallFunction|UpdateHealth))))

(event EventInRange
  (params (Nav :type Vector :default "0, 0, 0"))
  (bind (_x _y _z) (Math|Vector|BreakVector Nav))
  (bind _returnvalue (Transformation|GetActorLocation))
  (bind (_x_2 _y_2 _z_2) (Math|Vector|BreakVector _returnvalue))
  ;[1 1 1] Test for getting the enmies to jump
  (Character|LaunchCharacter (Math|Vector|MakeVector (|((NavX-LocationX)/{44C7B3E8-4CA0-6DB6-52F0-6EBAE0C273C1}) _x _x_2) (|((NavY-LocationY)/{44C7B3E8-4CA0-6DB6-52F0-6EBAE0C273C1}) _y _y_2) (|((DestintionHight-(StartHight-(((Power({44C7B3E8-4CA0-6DB6-52F0-6EBAE0C273C1},1))*1)*{7A1D24F7-4759-3692-F26B-B08FC70A065F})))/{44C7B3E8-4CA0-6DB6-52F0-6EBAE0C273C1}) _z _z_2)) true true))

(fn ConstructionScript)