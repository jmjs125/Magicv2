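; BP_MyNavLinkProxy is a nav link proxy that makes AI characters jump across its smart link.
; When an AiCharacter reaches the link, it is launched toward the destination, overriding its current horizontal and vertical velocity.
; CreateVelocity solves the ballistic launch vector from start, destination and the TimeLenght flight time, using a hardcoded gravity of 982 rather than the world's setting.
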(event EventBeginPlay)

(event Collision|EventActorBeginOverlap
  (params (OtherActor :type Actor%20Object%20Reference)))

(event EventTick
  (params (DeltaSeconds :type Float%20%28single-precision%29)))

(event EventSmartLinkReached
  (params (Agent :type Actor%20Object%20Reference) (Destination :type Vector%20%28by%20ref%29 :default "0, 0, 0"))
  ;[1 1 1] reaches the link
  (bind _asai_character (Utilities|Casting|CastToAiCharacter Agent))
  (bind _velocity (CallFunction|CreateVelocity Destination (Transformation|GetActorLocation _asai_character) (Variables|Default|GetTimeLenght)))
  (Character|LaunchCharacter _asai_character _velocity true true))

(fn ConstructionScript)

(fn CreateVelocity
  (params (DestinationLocation :type Vector) (Startinglocation :type Vector) (Time :type Float%20%28single-precision%29))
  (bind (_x _y _z) (Math|Vector|BreakVector DestinationLocation))
  (bind (_x_2 _y_2 _z_2) (Math|Vector|BreakVector Startinglocation))
  (LocalVariables|SetTimes Time)
  (return (Math|Vector|MakeVector (/ (- _x _x_2) (LocalVariables|GetTimes)) (/ (- _y _y_2) (LocalVariables|GetTimes)) (/ (- _z (+ _z_2 (* (Math|Float|Square (LocalVariables|GetTimes)) -0.5 982.0))) (LocalVariables|GetTimes)))))