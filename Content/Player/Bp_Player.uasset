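; Player character Blueprint that manages the shop and HUD widgets, shield and health display, and the death check.
; BeginPlay creates both widgets, and holding the Shop input shows the shop and cursor and stops active movement.
; Tick syncs BoxComponent and GroundAttackSpawner to Box1, then, without a shield, shows health over shield and calls PlayersDead at zero health.
; An end-game widget chain exists but is unconnected.
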(event EventBeginPlay
  (bind _returnvalue (UserInterface|CreateWidget "/Game/UI/Shop/Shop.Shop_C"))
  (Variables|Default|SetShop_0 _returnvalue)
  (bind _returnvalue_2 (UserInterface|CreateWidget "/Game/UI/Hud.Hud_C"))
  (Variables|Default|SetHud _returnvalue_2))

(event Collision|EventActorBeginOverlap
  (params (OtherActor :type Actor%20Object%20Reference)))

(event EventTick
  (params (DeltaSeconds :type Float%20%28single-precision%29))
  (bind _box1 (Variables|Default|GetBox1))
  (bind _hud (Variables|Default|GetHud))
  (bind _returnvalue (Transformation|GetWorldLocation _box1))
  (Utilities|FlowControl|Sequence
    (:then_0
      (Transformation|SetWorldLocationAndRotation (Variables|Default|GetBoxComponent) _returnvalue (Transformation|GetWorldRotation _box1) false false)
      (Transformation|SetWorldLocationAndRotation (Variables|Default|GetGroundAttackSpawner) _returnvalue "0, 0, 0" false false))
    (:then_2
      (if (not (Variables|Default|GetPlayerShield))
        (Widget|SetVisibility (Variables|/Game/UI/Hud.Hud_C|Getshield _hud) "Hidden")
        (Widget|SetVisibility (Variables|/Game/UI/Hud.Hud_C|GetHealth _hud) "Visible")
        (if (<= (Variables|Default|GetHealth) 0.0)
          (Class|MyCharacter|PlayersDead))))))

(event Input|ActionEvents|InputActionShop
  (params (Key :type Key%20Structure))
  (bind _returnvalue (Game|GetPlayerController 0))
  (bind _shop_0 (Variables|Default|GetShop_0))
  (:Pressed
    (UserInterface|Viewport|AddtoViewport _shop_0 0)
    (Variables|/Script/Engine.PlayerController|SetbShowMouseCursor _returnvalue true)
    (Class|NavMovementComponent|StopActiveMovement (Variables|Character|GetCharacterMovement self)))
  (:Released
    (Widget|RemovefromParent _shop_0)
    (Variables|/Script/Engine.PlayerController|SetbShowMouseCursor _returnvalue false)))

(fn ConstructionScript)